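; Player resource component for the building system that links a resource map to the main widget's UI and tracks the selected resource.
; InitManager has the player's main widget generate per-resource widgets, then fills in their amounts.
; UpdateResourceDisplay refreshes the matching amount, plus the current-resource display when that resource is selected and the player is in a specific state.
; SetNextResource cycles the selection with wraparound, updates the UI and calls OnResourceChanged.
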(event Custom|OnResourceChanged)

(event Custom|InitManager
  (params (PlayerReference :type Third%20Person%20Character%20Object%20Reference))
  (Utilities|IsValid PlayerReference
    (:Is%20Valid
      (Variables|Default|SetPlayerReference PlayerReference)
      (Variables|Default|SetInitialized? true)
      (bind _createdwidgets (Default|GenerateResourceWidget (Variables|/Game/ThirdPersonBP/Blueprints/ThirdPersonCharacter.ThirdPersonCharacter_C|GetmainWidget (Variables|Default|GetPlayerReference)) self))
      (Variables|Default|SetResourceWidgets _createdwidgets)
      (bind _keys (Utilities|Map|Keys (Variables|Default|GetResources)))
      (for _array_element _keys
        (CallFunction|UpdateResourceDisplay _array_element))
      (CallFunction|SetCurrentResource))))

(event EventBeginPlay
  (|CallParentFunction) ; This node is disabled and will not be called.\nDrag off pins to build functionality.
)

(event EventTick
  (params (DeltaSeconds :type Float%20%28single-precision%29))
  (|CallParentFunction DeltaSeconds) ; This node is disabled and will not be called.\nDrag off pins to build functionality.
)

(event EventUpdateResourceDisplay
  (params (Resource :type Bp%20Master%20Resource%20Class%20Reference))
  (bind _output_get (Variables|Default|SetLocalResource_0 Resource))
  (if (Variables|Default|GetInitialized?)
    (if (.Success? (CallFunction|GetWidgetforResource _output_get))
      (Rendering|Components|TextRender|SetText (Variables|/Game/Building_System/Widgets/W_Resource.W_Resource_C|GetAmount (.Widget (CallFunction|GetWidgetforResource _output_get))) (Utilities|Text|ToText(Integer) (CallFunction|GetResource (Variables|Default|GetLocalResource_0)) false false))
      (if (and (== (CallFunction|GetSelectedResource) (Variables|Default|GetLocalResource_0)) (Utilities|Enum|Equal(Enum) (Variables|/Game/ThirdPersonBP/Blueprints/ThirdPersonCharacter.ThirdPersonCharacter_C|GetState (Variables|Default|GetPlayerReference)) "NewEnumerator1"))
        (Default|UpdateCurrentResource (Variables|/Game/ThirdPersonBP/Blueprints/ThirdPersonCharacter.ThirdPersonCharacter_C|GetmainWidget (Variables|Default|GetPlayerReference)) self)))))

(fn GetSelectedIndex
  (return (Variables|Default|GetSelectedResourceIndex)))

(fn GetSelectedResource
  (bind _keys (Utilities|Map|Keys (Variables|Default|GetResources)))
  (return (Utilities|Array|Get(acopy) _keys (Variables|Default|GetSelectedResourceIndex))))

(fn GetWidgetforResource
  (params (Resource :type Bp%20Master%20Resource%20Class%20Reference))
  (bind _array_element (Utilities|Array|ForEachLoopwithBreak (Variables|Default|GetResourceWidgets) :!label _label)
    (:LoopBody
      (if (== (Variables|/Game/Building_System/Widgets/W_Resource.W_Resource_C|GetResource _array_element) Resource)
        (LocalVariables|SetWidgetFound _array_element)
        (goto _label Break)))
    (:Completed
      (Utilities|IsValid (LocalVariables|GetWidgetFound)
        (:Is%20Valid
          (return true (LocalVariables|GetWidgetFound)))
        (:Is%20Not%20Valid
          (return false 0))))))

(fn GetSelectedWidget
  (return (.Widget (CallFunction|GetWidgetforResource (CallFunction|GetSelectedResource)))))

(fn SetCurrentResource
  (Default|SelectResource (CallFunction|GetSelectedWidget) true false)
  (return))

(fn SetNextResource
  (Default|SelectResource (CallFunction|GetSelectedWidget) true false)
  (bind _keys (Utilities|Map|Keys (Variables|Default|GetResources)))
  (Variables|Default|SetSelectedResourceIndex (Math|Integer|SelectInt (+ (Variables|Default|GetSelectedResourceIndex) 1) 0 (< (Variables|Default|GetSelectedResourceIndex) (Utilities|Array|LastIndex _keys))))
  (CallFunction|SetCurrentResource)
  (Default|UpdateCurrentResource (Variables|/Game/ThirdPersonBP/Blueprints/ThirdPersonCharacter.ThirdPersonCharacter_C|GetmainWidget (Variables|Default|GetPlayerReference)) self)
  (CallFunction|OnResourceChanged))