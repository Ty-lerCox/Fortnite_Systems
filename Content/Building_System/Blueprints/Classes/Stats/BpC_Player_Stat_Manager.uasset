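; Player stat manager component that drives the player's HUD bars for stats such as Health and Shield.
; InitManager stores the player reference and runs stat setup, after which each stat key initializes its bar with that stat's value.
; UpdateStat pushes a stat's current value to its bar, which GetBarForStat selects from the player's main widget by stat type.
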(event Custom|InitManager
  (params (Player :type Third%20Person%20Character%20Object%20Reference))
  (Variables|Default|SetPlayerReference Player)
  (CallFunction|SetupStats))

(event EventOnStatSetup
  (bind _keys (Utilities|Map|Keys (Variables|Default|GetStats)))
  (for _array_element _keys
    (Default|InitializeBar (CallFunction|GetBarforStat _array_element) (.StatValue (CallFunction|GetStat _array_element)))))

(event EventUpdateStat
  (params (Stat :type e_Stats%20Enum :default "NewEnumerator0"))
  (Default|UpdateStat (CallFunction|GetBarforStat Stat) (.CurrentValue (CallFunction|GetStat Stat))))

(fn GetBarforStat
  (params (Stat :type e_Stats%20Enum :default "NewEnumerator0"))
  (bind _playerreference (Variables|Default|GetPlayerReference))
  (bind _mainwidget (Variables|/Game/ThirdPersonBP/Blueprints/ThirdPersonCharacter.ThirdPersonCharacter_C|GetmainWidget _playerreference))
  (return (Utilities|Select :Index Stat :NewEnumerator0 0 :NewEnumerator1 (Variables|/Game/Building_System/Widgets/W_Main.W_Main_C|GetSheildBar _mainwidget) :NewEnumerator2 (Variables|/Game/Building_System/Widgets/W_Main.W_Main_C|GetHealthBar _mainwidget) :NewEnumerator3 0)))