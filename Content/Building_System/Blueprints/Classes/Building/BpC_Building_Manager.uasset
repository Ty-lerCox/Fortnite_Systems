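; Building manager for the player's construction mode, handling building selection and a preview of the selected piece.
; Init generates building widgets through the main widget; selecting by index updates their highlight and switches the player from Combat to Construction.
; The selected class spawns with the player's chosen resource and is respawned when the selection changes.
; A looping timer moves it ahead of the player along the camera's forward vector, snapping position to a grid and yaw to increments.
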(event Custom|Init
  (params (PlayerReference :type Third%20Person%20Character%20Object%20Reference))
  (Utilities|IsValid PlayerReference
    (:Is%20Valid
      (Variables|Default|SetPlayerReference PlayerReference)
      (Variables|Default|SetInit? true)
      (bind _createdwidgets (Default|GenerateBuildingsWidget (Variables|/Game/ThirdPersonBP/Blueprints/ThirdPersonCharacter.ThirdPersonCharacter_C|GetmainWidget (Variables|Default|GetPlayerReference)) self))
      (Variables|Default|SetBuildingWidget _createdwidgets)
      (switch Utilities|FlowControl|Switch|Switchone_States (Variables|/Game/ThirdPersonBP/Blueprints/ThirdPersonCharacter.ThirdPersonCharacter_C|GetState (Variables|Default|GetPlayerReference))
        (:NewEnumerator1
          (CallFunction|SetCurrentBuilding true))))))

(event Custom|On%20Stop%20Building
  (if (Variables|Default|GetCurrentlyBuilding?)
    (Variables|Default|SetCurrentlyBuilding? false)
    (CallFunction|SetCurrentBuilding false)
    (Utilities|IsValid (Variables|Default|GetCurrentBuilding)
      (:Is%20Valid
        (Utilities|Time|ClearandInvalidateTimerbyHandle (Variables|Default|GetBuildingTimerHandle))
        (Actor|DestroyActor (Variables|Default|GetCurrentBuilding))
        (Variables|Default|SetCurrentBuilding 0)))))

(event Custom|On%20Start%20Building
  (if (Variables|Default|GetCurrentlyBuilding?)
    (CallFunction|ChangeCurrentBuilding)
    (else
      (CallFunction|StartBuilding)))
  (Variables|Default|SetCurrentlyBuilding? true))

(event Custom|BuildingTick
  (bind (_location _rotation) (CallFunction|GetBuildingPosandRot))
  (Transformation|SetActorLocationAndRotation (Variables|Default|GetCurrentBuilding) _location _rotation))

(event Custom|Start%20Building
  (bind (_location _rotation) (CallFunction|GetBuildingPosandRot))
  (bind _returnvalue (Game|SpawnActorfromClass (Utilities|Array|Get(acopy) (Variables|Default|GetBuildings) (Variables|Default|GetSelectedBuildingIndex)) (Math|Transform|MakeTransform _location _rotation "1,1,1") "Undefined" 0 (Default|GetSelectedResource (Variables|/Game/ThirdPersonBP/Blueprints/ThirdPersonCharacter.ThirdPersonCharacter_C|GetBpC_PlayerResources (Variables|Default|GetPlayerReference))) 0))
  (Variables|Default|SetCurrentBuilding _returnvalue)
  (bind _returnvalue_2 (Utilities|Time|SetTimerbyEvent (delegate Custom|BuildingTick) (Variables|Default|GetBuildingTickRate) true))
  (Variables|Default|SetBuildingTimerHandle _returnvalue_2))

(event Custom|Change%20Current%20Building
  (Utilities|Time|ClearandInvalidateTimerbyHandle (Variables|Default|GetBuildingTimerHandle))
  (Actor|DestroyActor (Variables|Default|GetCurrentBuilding))
  (Variables|Default|SetCurrentBuilding 0)
  (CallFunction|StartBuilding))

(fn GetWidgetforBuilding
  (params (Building :type Bp%20Master%20Building%20Class%20Reference))
  (bind _array_element (Utilities|Array|ForEachLoopwithBreak (Variables|Default|GetBuildingWidget) :!label _label)
    (:LoopBody
      (if (== (Variables|/Game/Building_System/Widgets/W_Building.W_Building_C|GetBuilding _array_element) Building)
        (LocalVariables|SetLocalFound _array_element)
        (goto _label Break)))
    (:Completed
      (Utilities|IsValid (LocalVariables|GetLocalFound)
        (:Is%20Valid
          (return true (LocalVariables|GetLocalFound)))
        (:Is%20Not%20Valid
          (return false 0))))))

(fn GetCurrentBuildingInfo
  (return (.BuildingData (Utilities|GetClassDefaults (Utilities|Array|Get(acopy) (Variables|Default|GetBuildings) (Variables|Default|GetSelectedBuildingIndex))))))

(fn SetCurrentBuilding
  (params (Select? :type Boolean))
  (bind _buildings (Variables|Default|GetBuildings))
  (bind _selectedbuildingindex (Variables|Default|GetSelectedBuildingIndex))
  (bind _output (Utilities|Array|Get(acopy) _buildings _selectedbuildingindex))
  (bind (_success_ _widget) (CallFunction|GetWidgetforBuilding _output))
  (if _success_
    (Default|SelectBuilding _widget Select?)
    (if Select?
      (CallFunction|OnStartBuilding)
      (return)
      (else
        (return)))
    (else
      (return))))

(fn SetBuildingbyIndex
  (params (Index :type Integer))
  (bind _output_get (LocalVariables|SetLocalIndex Index))
  (if (Math|Integer|InRange(Integer) _output_get 0 (Utilities|Array|LastIndex (Variables|Default|GetBuildings)))
    (switch Utilities|FlowControl|Switch|Switchone_States (Variables|/Game/ThirdPersonBP/Blueprints/ThirdPersonCharacter.ThirdPersonCharacter_C|GetState (Variables|Default|GetPlayerReference))
      (:NewEnumerator0
        (Variables|Default|SetSelectedBuildingIndex (LocalVariables|GetLocalIndex))
        (Default|ChangeState (Variables|Default|GetPlayerReference) "NewEnumerator1")
        (return))
      (:NewEnumerator1
        (if (!= (LocalVariables|GetLocalIndex) (Variables|Default|GetSelectedBuildingIndex))
          (CallFunction|SetCurrentBuilding false)
          (Variables|Default|SetSelectedBuildingIndex (LocalVariables|GetLocalIndex))
          (CallFunction|SetCurrentBuilding true)
          (return)
          (else
            (return)))))
    (else
      (return))))

(fn SettoGridLocation
  (params (in :type Vector))
  (bind (_x _y _z) (Math|Vector|BreakVector in))
  (bind _zgridsize (Variables|BuildingGrid|GetZGridSize))
  (bind _xgridsize (Variables|BuildingGrid|GetXGridSize))
  (bind _ygridsize (Variables|BuildingGrid|GetYGridSize))
  (return (Math|Vector|MakeVector (Math|Conversions|ToFloat(Integer) (* (Math|Float|Round (/ _x (Math|Conversions|ToFloat(Integer) _xgridsize))) _xgridsize)) (Math|Conversions|ToFloat(Integer) (* (Math|Float|Round (/ _y (Math|Conversions|ToFloat(Integer) _ygridsize))) _ygridsize)) (Math|Conversions|ToFloat(Integer) (* (Math|Float|Round (/ _z (Math|Conversions|ToFloat(Integer) _zgridsize))) _zgridsize)))))

(fn SettoSnapRotation
  (params (In :type Float%20%28single-precision%29))
  (bind _rotationsnap (Variables|BuildingGrid|GetRotationSnap))
  (return (* (Math|Float|Round (/ In (Math|Conversions|ToFloat(Integer) _rotationsnap))) _rotationsnap)))

(fn GetPlayerCastLocation
  (params (ForwardOffset :type Integer))
  (bind _playerreference (Variables|Default|GetPlayerReference))
  (return (+ (* (Math|Vector|GetForwardVector (Variables|/Game/ThirdPersonBP/Blueprints/ThirdPersonCharacter.ThirdPersonCharacter_C|GetFollowCamera _playerreference)) ForwardOffset) (Transformation|GetActorLocation _playerreference))))

(fn GetBuildingPosandRot
  (return (+ (CallFunction|SettoGridLocation (CallFunction|GetPlayerCastLocation (Variables|BuildingGrid|GetForwardBuildingOffset))) (Variables|BuildingGrid|GetLocationOffset)) (Math|Rotator|MakeRotator 0.0 0.0 (Math|Conversions|ToFloat(Integer) (+ (CallFunction|SettoSnapRotation (.Yaw (Math|Rotator|BreakRotator (Transformation|GetWorldRotation (Variables|/Game/ThirdPersonBP/Blueprints/ThirdPersonCharacter.ThirdPersonCharacter_C|GetFollowCamera (Variables|Default|GetPlayerReference)))))) (Variables|BuildingGrid|GetRotationOffset))))))